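; Actor Blueprint that holds save-state records for NPCs and chests, with no active event logic.
; AddSaveNPC searches NPCData by class, overwriting matches with the new row and shop data or appending an entry when none exists.
; AddSaveChest does the same on ChestData by ID and state, stopping at the first match, though its ArraySet shows no index input.
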(event EventBeginPlay)

(event Collision|EventActorBeginOverlap
  (params (OtherActor :type Actor%20Object%20Reference)))

(event EventTick
  (params (DeltaSeconds :type Float%20%28single-precision%29)))

(fn ConstructionScript)

(fn AddSaveNPC
  (params (Class :type BP%20NPC%20Class%20Reference) (Row :type String) (Shop :type Array%20of%20Product%20Structure%20Structures))
  (bind _npc_data (Variables|Default|GetNPC_Data))
  (for (_array_element _array_index) _npc_data
    (if (== (.Class (Utilities|Struct|BreakNPCStructure _array_element)) Class)
      (Utilities|Array|SetArrayElem _npc_data _array_index (Utilities|Struct|MakeNPCStructure Class Row Shop))
      (LocalVariables|SetIsAdd? true)))
  (if (not (LocalVariables|GetIsAdd?))
    (Utilities|Array|Add _npc_data (Utilities|Struct|MakeNPCStructure Class Row Shop))))

(fn AddSaveChest
  (params (ID :type Name) (State :type ChestState%20Enum :default "NewEnumerator2"))
  (bind _array_element (Utilities|Array|ForEachLoopwithBreak (Variables|Default|GetChest_Data) :!label _label)
    (:LoopBody
      (if (== (.ID (Utilities|Struct|BreakChestStructure _array_element)) ID)
        (Utilities|Array|SetArrayElem (Variables|Default|GetChest_Data) 0 (Utilities|Struct|MakeChestStructure ID State))
        (LocalVariables|SetIsAdd? true)
        (goto _label Break)))
    (:Completed
      (if (not (LocalVariables|GetIsAdd?))
        (Utilities|Array|Add (Variables|Default|GetChest_Data) (Utilities|Struct|MakeChestStructure ID State))))))