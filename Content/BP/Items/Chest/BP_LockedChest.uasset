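; BP_LockedChest is a chest that needs a BP_ChestKey from the player's inventory to open.
; When interacted with while Closed, it scans the inventory for the key class and records the slot of the last match.
; With a key, it overwrites that slot with an empty entry, plays a key sound and calls OpenChest.
; Without one, it hands the interaction to its dialogue component.
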(event EventBeginPlay
  (|CallParentFunction) ; This node is disabled and will not be called.\nDrag off pins to build functionality.
)

(event Collision|EventActorBeginOverlap
  (params (OtherActor :type Actor%20Object%20Reference))
  (|CallParentFunction OtherActor) ; This node is disabled and will not be called.\nDrag off pins to build functionality.
)

(event EventTick
  (params (DeltaSeconds :type Float%20%28single-precision%29))
  (|CallParentFunction DeltaSeconds) ; This node is disabled and will not be called.\nDrag off pins to build functionality.
)

(event EventInteract
  (params (PlayerRef :type BP%20Viking%20Object%20Reference) (Owner :type Object%20Object%20Reference))
  (bind _inventorycomponent (Variables|/Game/BP/Characters/Viking/BP_Viking.BP_Viking_C|GetInventoryComponent PlayerRef))
  (bind _inventory (Variables|/Game/BP/Inventory/InventoryComponent.InventoryComponent_C|GetInventory _inventorycomponent))
  (switch Utilities|FlowControl|Switch|SwitchonChestState (Variables|Default|GetState)
    (:NewEnumerator2
      (for (_array_element _array_index) _inventory
        (if (== (.ItemClass (Utilities|Struct|BreakItemStructure (.ItemStructure (Utilities|Struct|BreakSlotStrucutre _array_element)))) "/Game/BP/Items/BP_ChestKey.BP_ChestKey_C")
          (Variables|Default|SetHasKey? true)
          (Variables|Default|SetKeyIndex _array_index)))
      (if (Variables|Default|GetHasKey?)
        (Utilities|Array|SetArrayElem :TargetArray _inventory :Index (Variables|Default|GetKeyIndex))
        (Audio|PlaySound2D "/Game/Assets/Sound/Effects/Keys1_Cue.Keys1_Cue" 1.0 1.0 0.0 0 0)
        (CallFunction|OpenChest)
        (else
          (Default|Interact (Variables|Default|GetBP_DialogueComponent) PlayerRef self))))))

(fn ConstructionScript
  (|CallParentFunction))