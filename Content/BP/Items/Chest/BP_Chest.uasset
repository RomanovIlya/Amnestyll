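; Openable treasure chest with a Paper2D flipbook animation that rewards the player with either money or a spawned item.
; A sphere overlap shows a prompt widget to BP_Viking; Interact plays the opening animation once and lights a RectLight.
; Nonzero Money is credited with an on-screen notification; otherwise SpawnObjects is spawned.
; After a delay or the item's destruction, a timeline fades the dynamic material's opacity, then destroys the chest.
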(event OnComponentBeginOverlap(Sphere)
  (params (OverlappedComponent :type Primitive%20Component%20Object%20Reference) (OtherActor :type Actor%20Object%20Reference) (OtherComp :type Primitive%20Component%20Object%20Reference) (OtherBodyIndex :type Integer) (bFromSweep :type Boolean) (SweepResult :type Hit%20Result%20Structure%20%28by%20ref%29))
  (if (not (Variables|Default|GetIsOpened?))
    (Utilities|Casting|CastToBP_Viking OtherActor)
    (Rendering|SetVisibility (Variables|Default|GetWidget) true false)))

(event OnComponentEndOverlap(Sphere)
  (params (OverlappedComponent :type Primitive%20Component%20Object%20Reference) (OtherActor :type Actor%20Object%20Reference) (OtherComp :type Primitive%20Component%20Object%20Reference) (OtherBodyIndex :type Integer))
  (if (not (Variables|Default|GetIsOpened?))
    (Utilities|Casting|CastToBP_Viking OtherActor)
    (Rendering|SetVisibility (Variables|Default|GetWidget) false false)))

(event Custom|SelfDestroy
  (params (DestroyedActor :type Actor%20Object%20Reference))
  (bind _alpha (Timeline|Vanish Play)
    (:Update
      (Rendering|Material|SetScalarParameterValue (Variables|Default|GetMaterial) "Opacity" _alpha :!class /Script/Engine.MaterialInstanceDynamic))
    (:Finished
      (Actor|DestroyActor))))

(event Custom|OpenChest
  (bind _returnvalue (Transformation|GetActorLocation))
  (Variables|Default|SetIsOpened? true)
  (Rendering|SetVisibility (Variables|Default|GetWidget) false false)
  (Components|Timeline|PlayfromStart (Variables|Default|GetPaperFlipbook))
  (if (== (Variables|Default|GetMoney) 0)
    (bind _returnvalue_2 (Game|SpawnActorfromClass (Variables|Default|GetSpawnObjects) (Math|Transform|MakeTransform (Math|Vector|MakeVector (.x _returnvalue) (+ (.y _returnvalue) 2.0) (.z _returnvalue)) (Transformation|GetActorRotation) "1.000000,1.000000,1.000000") "AlwaysSpawn" "MultiplyWithRoot" 0 0))
    (Default|SpawnfromChest _returnvalue_2)
    (Rendering|Components|Light|SetIntensity (Variables|Default|GetRectLight) (Math|Float|Lerp 0.0 5e+03 1.0))
    (Game|BindEventtoOnDestroyed _returnvalue_2 (delegate Custom|SelfDestroy))
    (else
      (Variables|/Game/BP/Characters/Viking/BP_Viking.BP_Viking_C|SetMoney (stale EventInteract PlayerRef) (+ (Variables|/Game/BP/Characters/Viking/BP_Viking.BP_Viking_C|GetMoney (stale EventInteract PlayerRef)) (Variables|Default|GetMoney)))
      (bind _returnvalue_3 (UserInterface|CreateWidget "/Game/BP/Widget/WB_Notions.WB_Notions_C" (Game|GetPlayerController 0) (Utilities|Text|ToText(String) (Utilities|String|Append (Utilities|String|ToString(Text) (Utilities|Text|MakeLiteralText "Получено")) " " (Utilities|String|ToString(Integer) (Variables|Default|GetMoney)) " " (Utilities|String|ToString(Text) (Utilities|Text|MakeLiteralText "монет"))))))
      (UserInterface|Viewport|AddtoViewport _returnvalue_3 0)
      (Rendering|Components|Light|SetIntensity (Variables|Default|GetRectLight) (Math|Float|Lerp 0.0 5e+03 1.0))
      (Utilities|FlowControl|Delay 1.0)
      (CallFunction|SelfDestroy))))

(event EventBeginPlay
  (bind _paperflipbook (Variables|Default|GetPaperFlipbook))
  (Utilities|FlowControl|Sequence
    (:then_0
      (Sprite|SetFlipbook (Variables|Default|GetPaperFlipbook) (Variables|Default|GetSprite)))
    (:then_1
      (Components|Timeline|SetLooping _paperflipbook false)
      (Audio|Components|Audio|Stop _paperflipbook)
      (Class|PaperFlipbookComponent|SetPlaybackPositioninFrames _paperflipbook 0 false)
      (bind _returnvalue (Rendering|Material|CreateDynamicMaterialInstance (Variables|Default|GetPaperFlipbook) 0 "/Paper2D/MaskedLitSpriteMaterial.MaskedLitSpriteMaterial" "None" :!class /Script/Engine.PrimitiveComponent))
      (Variables|Default|SetMaterial _returnvalue))))

(event Collision|EventActorBeginOverlap
  (params (OtherActor :type Actor%20Object%20Reference)))

(event EventTick
  (params (DeltaSeconds :type Float%20%28single-precision%29)))

(event EventInteract
  (params (PlayerRef :type BP%20Viking%20Object%20Reference) (Owner :type Object%20Object%20Reference))
  (bind _returnvalue (Transformation|GetActorLocation))
  (if (not (Variables|Default|GetIsOpened?))
    (Variables|Default|SetIsOpened? true)
    (Rendering|SetVisibility (Variables|Default|GetWidget) false false)
    (Components|Timeline|PlayfromStart (Variables|Default|GetPaperFlipbook))
    (if (== (Variables|Default|GetMoney) 0)
      (bind _returnvalue_2 (Game|SpawnActorfromClass (Variables|Default|GetSpawnObjects) (Math|Transform|MakeTransform (Math|Vector|MakeVector (.x _returnvalue) (+ (.y _returnvalue) 2.0) (.z _returnvalue)) (Transformation|GetActorRotation) "1.000000,1.000000,1.000000") "AlwaysSpawn" "MultiplyWithRoot" 0 0))
      (Default|SpawnfromChest _returnvalue_2)
      (Rendering|Components|Light|SetIntensity (Variables|Default|GetRectLight) (Math|Float|Lerp 0.0 5e+03 1.0))
      (Game|BindEventtoOnDestroyed _returnvalue_2 (delegate Custom|SelfDestroy))
      (else
        (Variables|/Game/BP/Characters/Viking/BP_Viking.BP_Viking_C|SetMoney PlayerRef (+ (Variables|/Game/BP/Characters/Viking/BP_Viking.BP_Viking_C|GetMoney PlayerRef) (Variables|Default|GetMoney)))
        (bind _returnvalue_3 (UserInterface|CreateWidget "/Game/BP/Widget/WB_Notions.WB_Notions_C" (Game|GetPlayerController 0) (Utilities|Text|ToText(String) (Utilities|String|Append (Utilities|String|ToString(Text) (Utilities|Text|MakeLiteralText "Получено")) " " (Utilities|String|ToString(Integer) (Variables|Default|GetMoney)) " " (Utilities|String|ToString(Text) (Utilities|Text|MakeLiteralText "монет"))))))
        (UserInterface|Viewport|AddtoViewport _returnvalue_3 0)
        (Rendering|Components|Light|SetIntensity (Variables|Default|GetRectLight) (Math|Float|Lerp 0.0 5e+03 1.0))
        (Utilities|FlowControl|Delay 1.0)
        (CallFunction|SelfDestroy)))))

(fn ConstructionScript)