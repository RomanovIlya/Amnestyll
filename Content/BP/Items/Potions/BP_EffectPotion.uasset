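; Potion pickup item that grants a stat effect to the player Viking.
; Its PickUpBenefits override runs the parent check, then adds PotionStat to the Effects list on the player's health component and recalculates stats.
; It returns false without applying anything when the parent check fails, and all event graph nodes are disabled.
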(event EventBeginPlay
  (|CallParentFunction) ; This node is disabled and will not be called.\nDrag off pins to build functionality.
)

(event Collision|EventActorBeginOverlap
  (params (OtherActor :type Actor%20Object%20Reference))
  (|CallParentFunction OtherActor) ; This node is disabled and will not be called.\nDrag off pins to build functionality.
)

(event EventTick
  (params (DeltaSeconds :type Float%20%28single-precision%29))
  (|CallParentFunction DeltaSeconds) ; This node is disabled and will not be called.\nDrag off pins to build functionality.
)

(fn ConstructionScript
  (|CallParentFunction))

(fn PickUpBenefits
  (bind _success (|CallParentFunction))
  (if _success
    (bind _asbp_viking (Utilities|Casting|CastToBP_Viking (Game|Player|GetPlayerPawn 0)))
    (Utilities|Array|Add (Variables|/Game/BP/Component/BP_PlayerHealthComponent.BP_PlayerHealthComponent_C|GetEffects (Variables|/Game/BP/Characters/Viking/BP_Viking.BP_Viking_C|GetBP_PlayerHealthComponent _asbp_viking)) (Variables|Default|GetPotionStat))
    (Default|CalculateStats (Variables|/Game/BP/Characters/Viking/BP_Viking.BP_Viking_C|GetBP_PlayerHealthComponent _asbp_viking))
    (return true)
    (else
      (return false))))