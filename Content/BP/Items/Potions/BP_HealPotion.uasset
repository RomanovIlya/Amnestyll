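; Heal potion pickup item, a child Blueprint that overrides the parent's PickUpBenefits to heal the player.
; If the parent check succeeds, it casts player pawn 0 to BP_Viking and returns the result of HealCharacter on its health component.
; Otherwise it returns false; the event graph holds only disabled default nodes.
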(event EventBeginPlay
  (|CallParentFunction) ; This node is disabled and will not be called.\nDrag off pins to build functionality.
)

(event Collision|EventActorBeginOverlap
  (params (OtherActor :type Actor%20Object%20Reference))
  (|CallParentFunction OtherActor) ; This node is disabled and will not be called.\nDrag off pins to build functionality.
)

(event EventTick
  (params (DeltaSeconds :type Float%20%28single-precision%29))
  (|CallParentFunction DeltaSeconds) ; This node is disabled and will not be called.\nDrag off pins to build functionality.
)

(fn ConstructionScript
  (|CallParentFunction))

(fn PickUpBenefits
  (bind _success (|CallParentFunction))
  (if _success
    (bind _asbp_viking (Utilities|Casting|CastToBP_Viking (Game|Player|GetPlayerPawn 0)))
    (bind _success_2 (Default|HealCharacter (Variables|/Game/BP/Characters/Viking/BP_Viking.BP_Viking_C|GetBP_PlayerHealthComponent _asbp_viking)))
    (return _success_2)
    (else
      (return false))))