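; BP_TraiderRing is an interactable ring pickup from the trader item set that also advances the player's diary.
; On Interact it adds one item to the player's InventoryComponent, then runs PickUpBenefits, shows a "received" notification and destroys itself.
; The PickUpBenefits override updates the "Ring" diary state in GI_Sundered if the parent call succeeds.
; After the destroy call it passes itself to BP_SaveInst's CheckItems.
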(event EventBeginPlay
  (|CallParentFunction) ; This node is disabled and will not be called.\nDrag off pins to build functionality.
)

(event Collision|EventActorBeginOverlap
  (params (OtherActor :type Actor%20Object%20Reference))
  (|CallParentFunction OtherActor) ; This node is disabled and will not be called.\nDrag off pins to build functionality.
)

(event EventTick
  (params (DeltaSeconds :type Float%20%28single-precision%29))
  (|CallParentFunction DeltaSeconds) ; This node is disabled and will not be called.\nDrag off pins to build functionality.
)

(event EventInteract
  (params (PlayerRef :type BP%20Viking%20Object%20Reference) (Owner :type Object%20Object%20Reference))
  (Variables|/Game/BP/Characters/Viking/BP_Viking.BP_Viking_C|SetIsIntercting? PlayerRef false)
  (bind _succes (Default|AddtoInventory (Actor|GetComponentbyClass PlayerRef "/Game/BP/Inventory/InventoryComponent.InventoryComponent_C") (Utilities|Struct|MakeSlotStrucutre (Variables|Default|GetItemStrucutre) 1)))
  (if _succes
    (CallFunction|PickUpBenefits)
    (Default|NotionEvent PlayerRef (Utilities|Text|ToText(String) (Utilities|String|Append (Utilities|String|ToString(Text) (Utilities|Text|MakeLiteralText "Получено")) " x1 " (Utilities|String|ToString(Text) (.Itemname (Utilities|Struct|BreakItemStructure (Variables|Default|GetItemStrucutre)))))))
    (Actor|DestroyActor)
    (bind _outactors (Actor|GetAllActorsOfClass "/Game/BP/Save/BP_SaveInst.BP_SaveInst_C"))
    (Default|CheckItems (Utilities|Array|Get(acopy) _outactors) self)))

(fn ConstructionScript
  (|CallParentFunction))

(fn PickUpBenefits
  (bind _success (|CallParentFunction))
  (if _success
    (bind _asgi_sundered (Utilities|Casting|CastToGI_Sundered (Game|GetGameInstance)))
    (Default|UpdateDiaryState _asgi_sundered "Ring")
    (return true)))