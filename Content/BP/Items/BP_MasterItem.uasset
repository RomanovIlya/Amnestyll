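; Base pickup item that shows an interaction widget while a BP_Viking overlaps its sphere.
; Interact either adds one item to the player's InventoryComponent with a pickup notification or calls PickUpBenefits, destroying the actor on success.
; PickUpBenefits returns true here, apparently as a hook for child items.
; SpawnFromChest disables box physics and runs a timeline that scales and lifts the sprite.
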(event OnComponentBeginOverlap(Sphere)
  (params (OverlappedComponent :type Primitive%20Component%20Object%20Reference) (OtherActor :type Actor%20Object%20Reference) (OtherComp :type Primitive%20Component%20Object%20Reference) (OtherBodyIndex :type Integer) (bFromSweep :type Boolean) (SweepResult :type Hit%20Result%20Structure%20%28by%20ref%29))
  (Utilities|Casting|CastToBP_Viking OtherActor)
  (Rendering|SetVisibility (Variables|Default|GetWidgetInteraction) true false))

(event OnComponentEndOverlap(Sphere)
  (params (OverlappedComponent :type Primitive%20Component%20Object%20Reference) (OtherActor :type Actor%20Object%20Reference) (OtherComp :type Primitive%20Component%20Object%20Reference) (OtherBodyIndex :type Integer))
  (Utilities|Casting|CastToBP_Viking OtherActor)
  (Rendering|SetVisibility (Variables|Default|GetWidgetInteraction) false false))

(event Custom|SpawnFromChest
  (bind _papersprite (Variables|Default|GetPaperSprite))
  (Variables|Default|SetScale (Transformation|GetWorldScale (Variables|Default|GetPaperSprite)))
  (Physics|SetSimulatePhysics (Variables|Default|GetBox) false)
  (bind _alpha (Timeline|Offset Play)
    (:Update
      (Transformation|SetWorldScale3D _papersprite (Math|Vector|MakeVector (* _alpha (.x (Variables|Default|GetScale))) (* _alpha (.x (Variables|Default|GetScale))) (* _alpha (.x (Variables|Default|GetScale)))))
      (Transformation|AddLocalOffset _papersprite (Math|Vector|MakeVector 0.0 0.0 (* _alpha 3.0)) false false))))

(event EventBeginPlay)

(event Collision|EventActorBeginOverlap
  (params (OtherActor :type Actor%20Object%20Reference)))

(event EventTick
  (params (DeltaSeconds :type Float%20%28single-precision%29)))

(event EventInteract
  (params (PlayerRef :type BP%20Viking%20Object%20Reference) (Owner :type Object%20Object%20Reference))
  (bind _itemstrucutre (Variables|Default|GetItemStrucutre))
  (Variables|/Game/BP/Characters/Viking/BP_Viking.BP_Viking_C|SetIsIntercting? PlayerRef false)
  (if (.canbeadded _itemstrucutre)
    (bind _succes (Default|AddtoInventory (Actor|GetComponentbyClass PlayerRef "/Game/BP/Inventory/InventoryComponent.InventoryComponent_C") (Utilities|Struct|MakeSlotStrucutre (Variables|Default|GetItemStrucutre) 1)))
    (if _succes
      (Default|NotionEvent PlayerRef (Utilities|Text|ToText(String) (Utilities|String|Append (Utilities|String|ToString(Text) (Utilities|Text|MakeLiteralText "Получено")) " x1 " (Utilities|String|ToString(Text) (.Itemname (Utilities|Struct|BreakItemStructure (Variables|Default|GetItemStrucutre)))))))
      (Actor|DestroyActor :!label _label))
    (elif (.ispickupbenefitial _itemstrucutre)
      (bind _success (CallFunction|PickUpBenefits))
      (if _success
        (goto _label)))))

(fn ConstructionScript)

(fn PickUpBenefits
  (return true))