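; One-shot trigger volume that shows a guide popup when BP_Viking enters its box.
; The overlap creates WB_Guide with the trigger's media source, button word and description, then switches to UI-only input with a visible cursor.
; It freezes gameplay through zero global time dilation and destroys itself and every other BP_GuideTrigger sharing the same MediaSource, preventing repeat guides.
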(event OnComponentBeginOverlap(Box)
  (params (OverlappedComponent :type Primitive%20Component%20Object%20Reference) (OtherActor :type Actor%20Object%20Reference) (OtherComp :type Primitive%20Component%20Object%20Reference) (OtherBodyIndex :type Integer) (bFromSweep :type Boolean) (SweepResult :type Hit%20Result%20Structure%20%28by%20ref%29))
  (bind _returnvalue (Game|GetPlayerController 0))
  (Utilities|Casting|CastToBP_Viking OtherActor)
  (bind _returnvalue_2 (UserInterface|CreateWidget "/Game/BP/Widget/Guide/WB_Guide.WB_Guide_C" 0 (Variables|Default|GetMedia%20Source) (Variables|Default|GetButton%20Word) (Variables|Default|GetDescrip)))
  (UserInterface|Viewport|AddtoViewport _returnvalue_2 0)
  (Input|SetInputModeUIOnly _returnvalue _returnvalue_2 "DoNotLock" false)
  (Variables|/Script/Engine.PlayerController|SetbShowMouseCursor _returnvalue true)
  (Actor|DestroyActor)
  (Utilities|Time|SetGlobalTimeDilation 0.0)
  (bind _outactors (Actor|GetAllActorsOfClass "BP_GuideTrigger_C"))
  (for _array_element _outactors
    (if (== (Variables|BP_GuideTrigger_C|GetMedia%20Source _array_element) (Variables|Default|GetMedia%20Source))
      (Actor|DestroyActor _array_element))))

(event EventBeginPlay)

(event Collision|EventActorBeginOverlap
  (params (OtherActor :type Actor%20Object%20Reference)))

(event EventTick
  (params (DeltaSeconds :type Float%20%28single-precision%29)))

(fn ConstructionScript)