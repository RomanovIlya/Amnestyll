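; BP_DamageZone is a cave hazard volume that hurts the Viking player and sends them back to their last checkpoint.
; When a BP_Viking overlaps its box, it disables movement and applies a fixed amount of damage.
; If the Viking is not dead, a camera fade hides the teleport to LastCheckpoint, then clears as walking is restored.
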(event OnComponentBeginOverlap(Box)
  (params (OverlappedComponent :type Primitive%20Component%20Object%20Reference) (OtherActor :type Actor%20Object%20Reference) (OtherComp :type Primitive%20Component%20Object%20Reference) (OtherBodyIndex :type Integer) (bFromSweep :type Boolean) (SweepResult :type Hit%20Result%20Structure%20%28by%20ref%29))
  (bind _returnvalue (Game|GetPlayerCameraManager 0))
  (bind _asbp_viking (Utilities|Casting|CastToBP_Viking OtherActor))
  (Pawn|Components|CharacterMovement|DisableMovement (Variables|/Script/Engine.Character|GetCharacterMovement _asbp_viking))
  (Game|Damage|ApplyDamage _asbp_viking 25.0 0 self)
  (if (not (Variables|/Game/BP/Characters/Viking/BP_Viking.BP_Viking_C|GetIsDead? _asbp_viking))
    (CameraFades|StartCameraFade :self _returnvalue :ToAlpha 1.0 :Duration 0.2 :bHoldWhenFinished true)
    (Utilities|FlowControl|Delay 0.3)
    (Transformation|SetActorLocation _asbp_viking (Variables|/Game/BP/Characters/Viking/BP_Viking.BP_Viking_C|GetLastCheckpoint _asbp_viking) false false)
    (Utilities|FlowControl|Delay 0.2)
    (CameraFades|StopCameraFade _returnvalue)
    (Pawn|Components|CharacterMovement|SetMovementMode (Variables|/Script/Engine.Character|GetCharacterMovement _asbp_viking) "MOVE_Walking" 0)))

(event EventBeginPlay)

(event Collision|EventActorBeginOverlap
  (params (OtherActor :type Actor%20Object%20Reference)))

(event EventTick
  (params (DeltaSeconds :type Float%20%28single-precision%29)))

(fn ConstructionScript)