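; BP_Plate is a cave pressure plate that sinks when a BP_Viking steps on its box trigger.
; The Active timeline lowers the paper sprite, then sets IsActive and reports the PlateNumber through ActivePlate.
; DeactivePlate plays a second timeline that raises the sprite and clears IsActive, re-arming the plate.
; Both timelines add a local Z offset each update, so movement accumulates rather than interpolating between fixed positions.
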(event OnComponentBeginOverlap(Box)
  (params (OverlappedComponent :type Primitive%20Component%20Object%20Reference) (OtherActor :type Actor%20Object%20Reference) (OtherComp :type Primitive%20Component%20Object%20Reference) (OtherBodyIndex :type Integer) (bFromSweep :type Boolean) (SweepResult :type Hit%20Result%20Structure%20%28by%20ref%29))
  (if (not (Variables|Default|GetIsActive?))
    (Utilities|Casting|CastToBP_Viking OtherActor)
    (bind _alpha (Timeline|Active Play)
      (:Update
        (Transformation|AddLocalOffset (Variables|Default|GetPaperSprite1) (Math|Vector|MakeVector 0.0 0.0 (* _alpha -1.0)) false false))
      (:Finished
        (Variables|Default|SetIsActive? true)
        (Default|CallActivePlate (Variables|Default|GetPlateNumber))))))

(event Custom|DeactivePlate
  (bind _alpha (Timeline|Diactive Play)
    (:Update
      (Transformation|AddLocalOffset (Variables|Default|GetPaperSprite1) (Math|Vector|MakeVector 0.0 0.0 _alpha) false false))
    (:Finished
      (Variables|Default|SetIsActive? false))))

(event EventBeginPlay)

(event Collision|EventActorBeginOverlap
  (params (OtherActor :type Actor%20Object%20Reference)))

(event EventTick
  (params (DeltaSeconds :type Float%20%28single-precision%29)))

(fn ConstructionScript)