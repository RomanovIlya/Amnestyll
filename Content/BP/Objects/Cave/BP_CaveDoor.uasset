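; BP_CaveDoor is an interactable cave entrance that either shows dialogue when locked or moves the player into a streamed level.
; A trigger box shows or hides a prompt widget as the BP_Viking character enters or leaves.
; When unlocked, Interact fades the camera to black, loads the level, then disables movement and camera lag and teleports the player to the gate location.
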(event OnComponentBeginOverlap(Box)
  (params (OverlappedComponent :type Primitive%20Component%20Object%20Reference) (OtherActor :type Actor%20Object%20Reference) (OtherComp :type Primitive%20Component%20Object%20Reference) (OtherBodyIndex :type Integer) (bFromSweep :type Boolean) (SweepResult :type Hit%20Result%20Structure%20%28by%20ref%29))
  (Utilities|Casting|CastToBP_Viking OtherActor)
  (Rendering|SetVisibility (Variables|Default|GetWidget) true false))

(event OnComponentEndOverlap(Box)
  (params (OverlappedComponent :type Primitive%20Component%20Object%20Reference) (OtherActor :type Actor%20Object%20Reference) (OtherComp :type Primitive%20Component%20Object%20Reference) (OtherBodyIndex :type Integer))
  (Utilities|Casting|CastToBP_Viking OtherActor)
  (Rendering|SetVisibility (Variables|Default|GetWidget) false false))

(event EventBeginPlay)

(event Collision|EventActorBeginOverlap
  (params (OtherActor :type Actor%20Object%20Reference)))

(event EventTick
  (params (DeltaSeconds :type Float%20%28single-precision%29)))

(event EventInteract
  (params (PlayerRef :type BP%20Viking%20Object%20Reference) (Owner :type Object%20Object%20Reference))
  (if (Variables|Default|GetDoorLock?)
    (Default|Interact (Variables|Default|GetBP_DialogueComponent) PlayerRef Owner)
    (else
      (CameraFades|StartCameraFade :self (Game|GetPlayerCameraManager 0) :ToAlpha 1.0 :Duration 0.5 :bHoldWhenFinished true)
      (Utilities|FlowControl|Delay 0.6)
      (Class|GameplayStatics|LoadStreamLevelbySoftObjectPtr (Variables|Default|GetLevel) true false)
      (Pawn|Components|CharacterMovement|DisableMovement (Variables|/Script/Engine.Character|GetCharacterMovement PlayerRef))
      (Variables|/Script/Engine.SpringArmComponent|SetbEnableCameraLag (Variables|/Game/BP/Characters/Viking/BP_Viking.BP_Viking_C|GetSpringArm PlayerRef) false)
      (Transformation|SetActorLocation PlayerRef (Variables|Default|GetGateLocation) false true))))

(fn ConstructionScript)