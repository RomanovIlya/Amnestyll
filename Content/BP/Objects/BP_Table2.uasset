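; Interactable table that shows a prompt component to a nearby BP_Viking and starts dialogue on Interact through its BPDialogueComponent.
; Tick polls for the dialogue's end, then closes the message and creates a fade-in widget.
; After a further delay, it spawns BP_Mim at the first TargetPoint found in the level and destroys that point.
; It spawns BP_Block at the remaining TargetPoints and destroys itself.
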(event OnComponentBeginOverlap(Sphere)
  (params (OverlappedComponent :type Primitive%20Component%20Object%20Reference) (OtherActor :type Actor%20Object%20Reference) (OtherComp :type Primitive%20Component%20Object%20Reference) (OtherBodyIndex :type Integer) (bFromSweep :type Boolean) (SweepResult :type Hit%20Result%20Structure%20%28by%20ref%29))
  (Utilities|Casting|CastToBP_Viking OtherActor)
  (Rendering|SetVisibility (Variables|Default|GetWE) true false))

(event OnComponentEndOverlap(Sphere)
  (params (OverlappedComponent :type Primitive%20Component%20Object%20Reference) (OtherActor :type Actor%20Object%20Reference) (OtherComp :type Primitive%20Component%20Object%20Reference) (OtherBodyIndex :type Integer))
  (Utilities|Casting|CastToBP_Viking OtherActor)
  (Rendering|SetVisibility (Variables|Default|GetWE) false false))

(event EventBeginPlay)

(event Collision|EventActorBeginOverlap
  (params (OtherActor :type Actor%20Object%20Reference)))

(event EventTick
  (params (DeltaSeconds :type Float%20%28single-precision%29))
  (if (Variables|/Game/BP/Component/BP_DialogueComponent.BP_DialogueComponent_C|GetIs%20Dialogue%20End? (Variables|Default|GetBP_DialogueComponent))
    (Utilities|FlowControl|Delay 0.2)
    (Class|BPIInteract|EndInteract(Message) (Variables|Default|GetBP_DialogueComponent))
    (Utilities|FlowControl|Sequence
      (:then_0
        (Utilities|FlowControl|Delay 0.6)
        (bind _outactors (Actor|GetAllActorsOfClass "/Script/Engine.TargetPoint"))
        (Game|SpawnActorfromClass "/Game/BP/Characters/enemy/Mimic/BP_Mim.BP_Mim_C" (Transformation|GetActorTransform (Utilities|Array|Get(acopy) _outactors)) "Undefined" "MultiplyWithRoot" 0 0)
        (Actor|DestroyActor (Utilities|Array|Get(acopy) _outactors))
        (bind _outactors_2 (Actor|GetAllActorsOfClass "/Script/Engine.TargetPoint"))
        (for _array_element _outactors_2
          (Game|SpawnActorfromClass "/Game/BP/Objects/BP_Block.BP_Block_C" (Transformation|GetActorTransform _array_element) "Undefined" "MultiplyWithRoot" 0 0)
          (Actor|DestroyActor)))
      (:then_1
        (bind _returnvalue (UserInterface|CreateWidget "/Game/BP/Widget/WB_FadeInOut.WB_FadeInOut_C" (Game|GetPlayerController 0) true))
        (UserInterface|Viewport|AddtoViewport _returnvalue 0)))))

(event EventInteract
  (params (PlayerRef :type BP%20Viking%20Object%20Reference) (Owner :type Object%20Object%20Reference))
  (Class|BPIInteract|Interact(Message) (Variables|Default|GetBP_DialogueComponent) PlayerRef self))

(fn ConstructionScript)