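; BP_Campfire is an interactable campfire that gives the player access to a save screen.
; Its Sphere overlap shows or hides a Widget as a BP_Viking enters or leaves.
; Interact creates WB_SaveScreen with an autosave filename, player and campfire references, then enables the cursor and UI input and locks player movement.
; The HaveScreen flag blocks duplicate screens and is not cleared within this Blueprint.
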(event OnComponentBeginOverlap(Sphere)
  (params (OverlappedComponent :type Primitive%20Component%20Object%20Reference) (OtherActor :type Actor%20Object%20Reference) (OtherComp :type Primitive%20Component%20Object%20Reference) (OtherBodyIndex :type Integer) (bFromSweep :type Boolean) (SweepResult :type Hit%20Result%20Structure%20%28by%20ref%29))
  (Utilities|Casting|CastToBP_Viking OtherActor)
  (Rendering|SetVisibility (Variables|Default|GetWidget) true false))

(event OnComponentEndOverlap(Sphere)
  (params (OverlappedComponent :type Primitive%20Component%20Object%20Reference) (OtherActor :type Actor%20Object%20Reference) (OtherComp :type Primitive%20Component%20Object%20Reference) (OtherBodyIndex :type Integer))
  (Utilities|Casting|CastToBP_Viking OtherActor)
  (Rendering|SetVisibility (Variables|Default|GetWidget) false false))

(event EventBeginPlay)

(event Collision|EventActorBeginOverlap
  (params (OtherActor :type Actor%20Object%20Reference)))

(event EventTick
  (params (DeltaSeconds :type Float%20%28single-precision%29)))

(event EventInteract
  (params (PlayerRef :type BP%20Viking%20Object%20Reference) (Owner :type Object%20Object%20Reference))
  (bind _returnvalue (Game|GetPlayerController 0))
  (if (not (Variables|Default|GetHaveScreen?))
    (bind _output_get (Variables|Default|SetPlayer%20Ref PlayerRef))
    (bind _returnvalue_2 (UserInterface|CreateWidget "/Game/BP/Widget/Save/WB_SaveScreen.WB_SaveScreen_C" _returnvalue "autosave.json" _output_get self))
    (UserInterface|Viewport|AddtoViewport _returnvalue_2 0)
    (Input|SetInputModeGameandUI _returnvalue 0 "DoNotLock" true false)
    (Variables|/Script/Engine.PlayerController|SetbShowMouseCursor _returnvalue true)
    (Variables|/Game/BP/Characters/Viking/BP_Viking.BP_Viking_C|SetIsMovementLock? (Variables|Default|GetPlayer%20Ref) true)
    (Variables|Default|SetHaveScreen? true)))

(fn ConstructionScript)