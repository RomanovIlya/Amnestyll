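; BP_CameraBlock is a trigger volume that freezes the BP_Viking player's camera while the character is inside it.
; When the Viking enters the box, its SpringArm and Background components detach, keeping their world position so they stop following.
; On exit, both components reattach to the Viking's CapsuleComponent and snap back to it.
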(event OnComponentBeginOverlap(Box)
  (params (OverlappedComponent :type Primitive%20Component%20Object%20Reference) (OtherActor :type Actor%20Object%20Reference) (OtherComp :type Primitive%20Component%20Object%20Reference) (OtherBodyIndex :type Integer) (bFromSweep :type Boolean) (SweepResult :type Hit%20Result%20Structure%20%28by%20ref%29))
  (bind _asbp_viking (Utilities|Casting|CastToBP_Viking OtherActor))
  (Transformation|DetachFromComponent (Variables|/Game/BP/Characters/Viking/BP_Viking.BP_Viking_C|GetSpringArm _asbp_viking) "KeepWorld" "KeepRelative" "KeepWorld" false))

(event OnComponentEndOverlap(Box)
  (params (OverlappedComponent :type Primitive%20Component%20Object%20Reference) (OtherActor :type Actor%20Object%20Reference) (OtherComp :type Primitive%20Component%20Object%20Reference) (OtherBodyIndex :type Integer))
  (bind _asbp_viking (Utilities|Casting|CastToBP_Viking OtherActor))
  (Transformation|AttachComponentToComponent (Variables|/Game/BP/Characters/Viking/BP_Viking.BP_Viking_C|GetSpringArm _asbp_viking) (Variables|/Script/Engine.Character|GetCapsuleComponent _asbp_viking) "None" "SnapToTarget" "KeepRelative" "KeepWorld" true)
  (Transformation|AttachComponentToComponent (Variables|/Game/BP/Characters/Viking/BP_Viking.BP_Viking_C|GetBackground _asbp_viking) (Variables|/Script/Engine.Character|GetCapsuleComponent _asbp_viking) "None" "SnapToTarget" "KeepRelative" "KeepWorld" true))

(event EventBeginPlay)

(event Collision|EventActorBeginOverlap
  (params (OtherActor :type Actor%20Object%20Reference)))

(event EventTick
  (params (DeltaSeconds :type Float%20%28single-precision%29)))

(fn ConstructionScript)