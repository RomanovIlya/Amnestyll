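; BP_MapTrigger3 is a map trigger that gates Box1, likely a blocker, on dialogue progress with two NPCs.
; When BP_Viking overlaps Box, it reads the Blacksmith and Barmaid dialogue row names as integers to gauge progress.
; If both exceed their thresholds it destroys Box1; otherwise it starts its own dialogue component's message.
; Interact also forwards to that dialogue component, only when IsDialogueEnd is true.
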(event OnComponentBeginOverlap(Box)
  (params (OverlappedComponent :type Primitive%20Component%20Object%20Reference) (OtherActor :type Actor%20Object%20Reference) (OtherComp :type Primitive%20Component%20Object%20Reference) (OtherBodyIndex :type Integer) (bFromSweep :type Boolean) (SweepResult :type Hit%20Result%20Structure%20%28by%20ref%29))
  (bind _asbp_viking (Utilities|Casting|CastToBP_Viking OtherActor))
  (bind _returnvalue (Actor|GetActorOfClass "/Game/BP/Characters/NPC/BP_Blacksmith.BP_Blacksmith_C"))
  (bind _returnvalue_2 (Actor|GetActorOfClass "/Game/BP/Characters/NPC/BP_Barmaid.BP_Barmaid_C"))
  (if (and (> (Math|Conversions|ToInteger(Byte) (Utilities|String|ToString(Name) (Variables|/Game/BP/Component/BP_DialogueComponent.BP_DialogueComponent_C|GetRowName (Variables|/Game/BP/Characters/NPC/BP_NPC.BP_NPC_C|GetBP_DialogueComponent _returnvalue_2)))) 20) (> (Math|Conversions|ToInteger(Byte) (Utilities|String|ToString(Name) (Variables|/Game/BP/Component/BP_DialogueComponent.BP_DialogueComponent_C|GetRowName (Variables|/Game/BP/Characters/NPC/BP_NPC.BP_NPC_C|GetBP_DialogueComponent _returnvalue)))) 14))
    (Components|DestroyComponent (Variables|Default|GetBox1))
    (else
      (Class|BPIInteract|Interact(Message) (Variables|Default|GetBP_DialogueComponent) _asbp_viking self))))

(event EventBeginPlay)

(event Collision|EventActorBeginOverlap
  (params (OtherActor :type Actor%20Object%20Reference)))

(event EventTick
  (params (DeltaSeconds :type Float%20%28single-precision%29)))

(event EventInteract
  (params (PlayerRef :type BP%20Viking%20Object%20Reference) (Owner :type Object%20Object%20Reference))
  (if (Variables|/Game/BP/Component/BP_DialogueComponent.BP_DialogueComponent_C|GetIs%20Dialogue%20End? (Variables|Default|GetBP_DialogueComponent))
    (Class|BPIInteract|Interact(Message) (Variables|Default|GetBP_DialogueComponent) PlayerRef self)))

(fn ConstructionScript)