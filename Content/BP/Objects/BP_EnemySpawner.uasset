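; Trigger-volume enemy spawner that locks the BP_Viking into an arena battle until every spawned enemy is destroyed.
; On overlap it spawns each class in Actors at a random reachable X within Radius, keeping its own Y and Z.
; It then shows two flipbooks and, after a short delay, makes two boxes block.
; OnDestroyed callbacks count down survivors, then reopen the barriers, end the Viking's battle state and destroy the spawner.
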(event OnComponentBeginOverlap(Box)
  (params (OverlappedComponent :type Primitive%20Component%20Object%20Reference) (OtherActor :type Actor%20Object%20Reference) (OtherComp :type Primitive%20Component%20Object%20Reference) (OtherBodyIndex :type Integer) (bFromSweep :type Boolean) (SweepResult :type Hit%20Result%20Structure%20%28by%20ref%29))
  (bind _returnvalue (Transformation|GetActorLocation))
  (bind (_x _y _z) (Math|Vector|BreakVector _returnvalue))
  (bind _asbp_viking (Utilities|Casting|CastToBP_Viking OtherActor))
  (Variables|Default|SetAs%20BP%20Viking _asbp_viking)
  (if (Variables|Default|GetIsBattleOver?)
    (Utilities|FlowControl|Sequence
      (:then_0
        (Variables|/Game/BP/Characters/Viking/BP_Viking.BP_Viking_C|SetIsInBattle? (Variables|Default|GetAs%20BP%20Viking) true)
        (Variables|Default|SetIsBattleOver? false)
        (for _array_element (Variables|Default|GetActors)
          (bind _randomlocation (AI|Navigation|GetRandomReachablePointinRadius _returnvalue (Variables|Default|GetRadius) 0 0))
          (bind _returnvalue_2 (Game|SpawnActorfromClass _array_element (Math|Transform|MakeTransform (Math|Vector|MakeVector (.x _randomlocation) _y _z) "0, 0, 0" "1.000000,1.000000,1.000000") "AlwaysSpawn" "MultiplyWithRoot" 0 0))
          (Utilities|Array|Add (Variables|Default|GetEnemyList) _returnvalue_2)
          (Variables|Default|SetActorNum (Utilities|Array|Length (Variables|Default|GetEnemyList)))))
      (:then_1
        (Utilities|FlowControl|Delay 0.2)
        (Collision|SetCollisionResponsetoAllChannels (Variables|Default|GetBox1) "ECR_Block")
        (Collision|SetCollisionResponsetoAllChannels (Variables|Default|GetBox2) "ECR_Block"))
      (:then_2
        (Rendering|SetVisibility (Variables|Default|GetPaperFlipbook) true false))
      (:then_3
        (for _array_element_2 (Variables|Default|GetEnemyList)
          (Game|BindEventtoOnDestroyed _array_element_2 (delegate Custom|OnDead)))))))

(event Custom|OnDead
  (params (DestroyedActor :type Actor%20Object%20Reference))
  (if (not (Variables|Default|GetIsBattleOver?))
    (bind _output_get (Variables|Default|SetActorNum (- (Variables|Default|GetActorNum) 1)))
    (if (not (> _output_get 0))
      (Variables|Default|SetIsBattleOver? true)
      (Collision|SetCollisionResponsetoAllChannels (Variables|Default|GetBox1) "ECR_Overlap")
      (Collision|SetCollisionResponsetoAllChannels (Variables|Default|GetBox2) "ECR_Overlap")
      (Rendering|SetVisibility (Variables|Default|GetPaperFlipbook) false false)
      (Variables|/Game/BP/Characters/Viking/BP_Viking.BP_Viking_C|SetIsInBattle? (Variables|Default|GetAs%20BP%20Viking) false)
      (Actor|DestroyActor))))

(event EventBeginPlay)

(event Collision|EventActorBeginOverlap
  (params (OtherActor :type Actor%20Object%20Reference)))

(event EventTick
  (params (DeltaSeconds :type Float%20%28single-precision%29)))

(fn ConstructionScript)