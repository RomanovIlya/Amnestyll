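; Dialogue component that runs branching, data-table-driven conversations between the player and its owner, such as an NPC.
; Each Interact shows the current row in WB_Dialogue, fires any trigger on the owner and stores the next row and table.
; Rows can spawn WB_Option choices that branch through OptionSelected; NeedSave records NPC progress and shop items via BP_SaveInst.
; Player movement and attacks stay locked until EndDialogue restores them.
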(event Custom|OptionSelected
  (params (DataTable :type Data%20Table%20Object%20Reference) (RowName :type Name))
  (bind _returnvalue (Utilities|GetDataTableRow DataTable RowName)
    (:then
      (Widget|Panel|ClearChildren (Variables|/Game/BP/Widget/WB_Dialogue.WB_Dialogue_C|GetOptionBox (Variables|Default|GetWidgetDialogue)))
      (Default|UpdateDialogue (Variables|Default|GetWidgetDialogue) (.Dialogue (Utilities|Struct|BreakDialogue_Structure _returnvalue)))
      (if (!= (.TriggerName (Utilities|Struct|BreakDialogue_Structure _returnvalue)) "")
        (Class|BPITrigger|Trigger(Message) (Variables|Default|GetOwner) (.TriggerName (Utilities|Struct|BreakDialogue_Structure _returnvalue)) (.Row (Utilities|Struct|BreakDialogue_Structure _returnvalue)) (.DataTable (Utilities|Struct|BreakDialogue_Structure _returnvalue))))
      (Variables|Default|SetRowName (.Row (Utilities|Struct|BreakDialogue_Structure _returnvalue)))
      (Variables|Default|SetDataTable (.DataTable (Utilities|Struct|BreakDialogue_Structure _returnvalue)))
      (Variables|Default|SetIs%20Dialogue%20End? (.IsDialogueEnd? (Utilities|Struct|BreakDialogue_Structure _returnvalue)))
      (Variables|Default|SetHasOption? false)
      (if (.OpenedDialogue? (Utilities|Struct|BreakDialogue_Structure _returnvalue))
        (CallFunction|UpdateOption (.DialogueOptions (Utilities|Struct|BreakDialogue_Structure _returnvalue)))))))

(event Custom|UpdateOption
  (params (Array :type Array%20of%20Optional%20Dialogue%20Structure%20Structures))
  (if (not (Variables|Default|GetHasOption?))
    (for _array_element Array
      (Variables|Default|SetHasOption? true)
      (bind _returnvalue (UserInterface|CreateWidget "/Game/BP/Widget/WB_Option.WB_Option_C" (Game|GetPlayerController 0) (.OptionName (Utilities|Struct|BreakOptionalDialogue_Structure _array_element)) self (.Database (Utilities|Struct|BreakOptionalDialogue_Structure _array_element)) (.Row (Utilities|Struct|BreakOptionalDialogue_Structure _array_element)) (.TriggerName (Utilities|Struct|BreakOptionalDialogue_Structure _array_element)) (Variables|Default|GetOwner)))
      (Widget|Panel|AddChild (Variables|/Game/BP/Widget/WB_Dialogue.WB_Dialogue_C|GetOptionBox (Variables|Default|GetWidgetDialogue)) _returnvalue))))

(event EventBeginPlay
  (Variables|Default|SetWidgetDialogue 0))

(event EventTick
  (params (DeltaSeconds :type Float%20%28single-precision%29)))

(event EventInteract
  (params (PlayerRef :type BP%20Viking%20Object%20Reference) (Owner :type Object%20Object%20Reference))
  (bind _returnvalue (Game|GetPlayerController 0))
  (Variables|Default|SetOwner Owner)
  (if (Variables|Default|GetIs%20Dialogue%20End?)
    (|EndDialogue PlayerRef)
    (else
      (Utilities|FlowControl|Sequence
        (:then_0
          (Utilities|IsValid (Variables|Default|GetWidgetDialogue)
            (:Is%20Valid
              (bind _returnvalue_2 (Utilities|GetDataTableRow (Variables|Default|GetDataTable) (Variables|Default|GetRowName))
                (:then
                  (Default|UpdateDialogue (Variables|Default|GetWidgetDialogue) (.Dialogue (Utilities|Struct|BreakDialogue_Structure _returnvalue_2)))
                  (if (!= (.TriggerName (Utilities|Struct|BreakDialogue_Structure _returnvalue_2)) "")
                    (Class|BPITrigger|Trigger(Message) (Variables|Default|GetOwner) (.TriggerName (Utilities|Struct|BreakDialogue_Structure _returnvalue_2)) (.Row (Utilities|Struct|BreakDialogue_Structure _returnvalue_2)) (.DataTable (Utilities|Struct|BreakDialogue_Structure _returnvalue_2))))
                  (Variables|Default|SetRowName (.Row (Utilities|Struct|BreakDialogue_Structure _returnvalue_2)))
                  (Variables|Default|SetDataTable (.DataTable (Utilities|Struct|BreakDialogue_Structure _returnvalue_2)))
                  (Variables|Default|SetIs%20Dialogue%20End? (.IsDialogueEnd? (Utilities|Struct|BreakDialogue_Structure _returnvalue_2)))
                  (if (.OpenedDialogue? (Utilities|Struct|BreakDialogue_Structure _returnvalue_2))
                    (CallFunction|UpdateOption (.DialogueOptions (Utilities|Struct|BreakDialogue_Structure _returnvalue_2)))))))
            (:Is%20Not%20Valid
              (bind _returnvalue_3 (Utilities|GetDataTableRow (Variables|Default|GetDataTable) (Variables|Default|GetRowName))
                (:then
                  (bind _returnvalue_4 (UserInterface|CreateWidget "/Game/BP/Widget/WB_Dialogue.WB_Dialogue_C" (Game|GetPlayerController 0) (Variables|Default|GetName) (.Dialogue (Utilities|Struct|BreakDialogue_Structure _returnvalue_3))))
                  (bind _output_get (Variables|Default|SetWidgetDialogue _returnvalue_4))
                  (UserInterface|Viewport|AddtoViewport _output_get 0)
                  (Input|SetInputModeGameandUI _returnvalue 0 "DoNotLock" true false)
                  (Variables|/Script/Engine.PlayerController|SetbShowMouseCursor _returnvalue true)
                  (if (!= (.TriggerName (Utilities|Struct|BreakDialogue_Structure _returnvalue_3)) "")
                    (Class|BPITrigger|Trigger(Message) (Variables|Default|GetOwner) (.TriggerName (Utilities|Struct|BreakDialogue_Structure _returnvalue_3)) (.Row (Utilities|Struct|BreakDialogue_Structure _returnvalue_3)) (.DataTable (Utilities|Struct|BreakDialogue_Structure _returnvalue_3))))
                  (Variables|Default|SetRowName (.Row (Utilities|Struct|BreakDialogue_Structure _returnvalue_3)))
                  (Variables|Default|SetDataTable (.DataTable (Utilities|Struct|BreakDialogue_Structure _returnvalue_3)))
                  (Variables|Default|SetIs%20Dialogue%20End? (.IsDialogueEnd? (Utilities|Struct|BreakDialogue_Structure _returnvalue_3)))
                  (if (.OpenedDialogue? (Utilities|Struct|BreakDialogue_Structure _returnvalue_3))
                    (CallFunction|UpdateOption (.DialogueOptions (Utilities|Struct|BreakDialogue_Structure _returnvalue_3))))))))
          (if (Variables|Default|GetNeedSave?)
            (bind _outactors (Actor|GetAllActorsOfClass "/Game/BP/Save/BP_SaveInst.BP_SaveInst_C"))
            (bind _asbp_npc (Utilities|Casting|CastToBP_NPC (Variables|Default|GetOwner)))
            (Default|AddSaveNPC (Utilities|Array|Get(acopy) _outactors) (Utilities|GetClass _asbp_npc) (Utilities|String|ToString(Name) (Variables|Default|GetRowName)) (Variables|/Game/BP/Component/BP_ShopComponent.BP_ShopComponent_C|GetItems (Variables|/Game/BP/Characters/NPC/BP_NPC.BP_NPC_C|GetBP_ShopComponent _asbp_npc)))))
        (:then_1
          (Variables|/Game/BP/Characters/Viking/BP_Viking.BP_Viking_C|SetIsMovementLock? PlayerRef true)
          (Variables|/Game/BP/Characters/Viking/BP_Viking.BP_Viking_C|SetCanAttack? PlayerRef false)
          (Variables|/Game/BP/Characters/Viking/BP_Viking.BP_Viking_C|SetIsDashing? PlayerRef true)
          (Pawn|Components|CharacterMovement|DisableMovement (Variables|/Script/Engine.Character|GetCharacterMovement PlayerRef))
          (Variables|/Game/BP/Characters/Viking/BP_Viking.BP_Viking_C|SetIsIntercting? PlayerRef true))))))

(event EventEndInteract
  (Utilities|IsValid (Variables|Default|GetWidgetDialogue)
    (:Is%20Valid
      (|EndDialogue (stale EventInteract PlayerRef)))))