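; Shop component that sells stocked items to the player's BP_Viking for money or, when the price is zero, for barter items.
; BeginPlay fills each product's item data from class defaults, and CreateShop builds a WB_Shop widget with one WB_Product per entry.
; Buy deducts payment without checking money, then adds the item to the inventory or spawns it nearby if that fails.
; It then decrements stock, refreshes the calling object and fires buy dispatchers.
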(event EventBeginPlay
  (for (_array_element _array_index) (Variables|Default|GetItems)
    (Utilities|Array|SetArrayElem (Variables|Default|GetItems) _array_index (Utilities|Struct|MakeProductStructure (.ItemStrucutre (Utilities|GetClassDefaults (Utilities|Array|Get(acopy) (Variables|Default|GetB_Item) _array_index))) (.Quantity (Utilities|Struct|BreakProductStructure _array_element)) (.ItemsValue (Utilities|Struct|BreakProductStructure _array_element)) (.Value (Utilities|Struct|BreakProductStructure _array_element))))))

(event EventTick
  (params (DeltaSeconds :type Float%20%28single-precision%29)))

(fn Buy
  (params (Object :type WB%20Product%20Object%20Reference) (Item :type Item%20Structure%20Structure) (ItemsValue :type Array%20of%20Slot%20Strucutre%20Structures) (Value :type Integer))
  (bind _asbp_viking (Utilities|Casting|CastToBP_Viking (Game|Player|GetPlayerPawn 0)))
  (if (== Value 0)
    (Default|MaxStack (Variables|/Game/BP/Characters/Viking/BP_Viking.BP_Viking_C|GetInventoryComponent _asbp_viking))
    (for _array_element ItemsValue
      (bind (_array_element_2 _array_index) (Utilities|Array|ForEachLoopwithBreak (Variables|/Game/BP/Inventory/InventoryComponent.InventoryComponent_C|GetInventory (Variables|/Game/BP/Characters/Viking/BP_Viking.BP_Viking_C|GetInventoryComponent _asbp_viking)) :!label _label)
        (:LoopBody
          (if (and (== (.ItemClass (Utilities|Struct|BreakItemStructure (.ItemStructure (Utilities|Struct|BreakSlotStrucutre _array_element_2)))) (.ItemClass (Utilities|Struct|BreakItemStructure (.ItemStructure (Utilities|Struct|BreakSlotStrucutre _array_element))))) (>= (.Qantity (Utilities|Struct|BreakSlotStrucutre _array_element_2)) (.Qantity (Utilities|Struct|BreakSlotStrucutre _array_element))))
            (if (> (- (.Qantity (Utilities|Struct|BreakSlotStrucutre _array_element_2)) (.Qantity (Utilities|Struct|BreakSlotStrucutre _array_element))) 0)
              (Utilities|Array|SetArrayElem (Variables|/Game/BP/Inventory/InventoryComponent.InventoryComponent_C|GetInventory (Variables|/Game/BP/Characters/Viking/BP_Viking.BP_Viking_C|GetInventoryComponent _asbp_viking)) _array_index (Utilities|Struct|MakeSlotStrucutre (.ItemStructure (Utilities|Struct|BreakSlotStrucutre _array_element_2)) (- (.Qantity (Utilities|Struct|BreakSlotStrucutre _array_element_2)) (.Qantity (Utilities|Struct|BreakSlotStrucutre _array_element)))))
              (goto _label Break)
              (else
                (Utilities|Array|SetArrayElem :TargetArray (Variables|/Game/BP/Inventory/InventoryComponent.InventoryComponent_C|GetInventory (Variables|/Game/BP/Characters/Viking/BP_Viking.BP_Viking_C|GetInventoryComponent _asbp_viking)) :Index _array_index)
                (goto _label Break)))))))
    (else
      (Variables|/Game/BP/Characters/Viking/BP_Viking.BP_Viking_C|SetMoney _asbp_viking (- (Variables|/Game/BP/Characters/Viking/BP_Viking.BP_Viking_C|GetMoney _asbp_viking) Value))))
  (|SpawnItem (Variables|/Game/BP/Characters/Viking/BP_Viking.BP_Viking_C|GetInventoryComponent _asbp_viking) _asbp_viking))

(fn CreateShop
  (params (CanBeClose? :type Boolean))
  (bind _returnvalue (Game|GetPlayerController 0))
  (bind _returnvalue_2 (UserInterface|CreateWidget "/Game/BP/Widget/Shops/WB_Shop.WB_Shop_C" _returnvalue CanBeClose?))
  (Variables|Default|SetShop _returnvalue_2)
  (UserInterface|Viewport|AddtoViewport _returnvalue_2 0)
  (Input|SetInputModeUIOnly _returnvalue _returnvalue_2 "DoNotLock" false)
  (Variables|/Script/Engine.PlayerController|SetbShowMouseCursor _returnvalue true)
  (for _array_element (Variables|Default|GetItems)
    (bind _returnvalue_3 (UserInterface|CreateWidget "/Game/BP/Widget/Shops/WB_Product.WB_Product_C" 0 (.Item (Utilities|Struct|BreakProductStructure _array_element)) (.ItemsValue (Utilities|Struct|BreakProductStructure _array_element)) (.Value (Utilities|Struct|BreakProductStructure _array_element)) (.Quantity (Utilities|Struct|BreakProductStructure _array_element)) self))
    (Widget|Panel|AddChild (Variables|/Game/BP/Widget/Shops/WB_Shop.WB_Shop_C|GetScrollBox_0 (Variables|Default|GetShop)) _returnvalue_3)))

(fn DestroyShop
  (Widget|RemovefromParent (Variables|Default|GetShop))
  (Variables|Default|SetShop 0)
  (Input|SetInputModeGameandUI (Game|GetPlayerController 0) 0 "DoNotLock" true false))