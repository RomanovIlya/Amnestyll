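; Player stat component for the Viking character, handling health, stamina, damage, defense and invulnerability time.
; CalculateStats sums equipped-item flat and percent bonuses onto base stats without resetting totals, preserving current health and stamina ratios.
; GetDamage applies diminishing-returns defense mitigation, HealCharacter spends limited charges to restore quarter health, and ConsumeStamina timestamps each use.
; After a delay, Tick sets stamina to a clamped per-frame amount rather than adding it.
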(event EventBeginPlay)

(event EventTick
  (params (DeltaSeconds :type Float%20%28single-precision%29))
  (if (and (< (Variables|Default|GetCurrentStamina) (Variables|Default|GetFinalStamina)) (>= (- (Utilities|Time|GetGameTimeinSeconds) (Variables|Default|GetLastStaminaUse)) (Variables|Default|GetStaminaRegenDelay)))
    (Variables|Default|SetCurrentStamina (Math|Float|Clamp(Float) (* DeltaSeconds 15.0) 0.0 (Variables|Default|GetFinalStamina)))))

(fn CalculateStats
  (LocalVariables|SetDeferencePercentHealth (/ (Variables|Default|GetCurrentHealth) (Variables|Default|GetFinalMaxHealth)))
  (LocalVariables|SetDeferencePercentStamina (/ (Variables|Default|GetCurrentStamina) (Variables|Default|GetFinalStamina)))
  (bind _asbp_viking (Utilities|Casting|CastToBP_Viking (Game|Player|GetPlayerPawn 0)))
  (for _array_element (Variables|/Game/BP/Inventory/InventoryComponent.InventoryComponent_C|GetEquipmentSlots (Variables|/Game/BP/Characters/Viking/BP_Viking.BP_Viking_C|GetInventoryComponent _asbp_viking))
    (|AddBonus _array_element))
  (Variables|Default|SetFinalMaxHealth (+ (+ (Variables|Default|GetBaseHealth) (LocalVariables|GetTotalHealthFlatBonus)) (* (Variables|Default|GetBaseHealth) (/ (LocalVariables|GetTotalHealthPercentBonus) 1e+02))))
  (Variables|Default|SetFinalDamage (+ (+ (Variables|Default|GetBaseDamage) (LocalVariables|GetTotalDamageFlatBonus)) (* (Variables|Default|GetBaseDamage) (/ (LocalVariables|GetTotalDamagePercentBonus) 1e+02))))
  (Variables|Default|SetFinalDefense (+ (+ (Variables|Default|GetBaseDefense) (LocalVariables|GetTotalDefenseFlatBonus)) (* (Variables|Default|GetBaseDefense) (/ (LocalVariables|GetTotalDefensePercentBonus) 1e+02))))
  (Variables|Default|SetFinalStamina (+ (+ (Variables|Default|GetBaseStamina) (LocalVariables|GetTotalStaminaFlatBonus)) (* (Variables|Default|GetBaseStamina) (/ (LocalVariables|GetTotalStaminaPercentBonus) 1e+02))))
  (Variables|Default|SetFinalInvulnerabilityTime (+ (Variables|Default|GetBaseInvulnerabilityTime) (LocalVariables|GetTotalInvulnerabilityFlatBonus)))
  (Utilities|FlowControl|Sequence
    (:then_0
      (Variables|Default|SetCurrentHealth (* (Variables|Default|GetFinalMaxHealth) (LocalVariables|GetDeferencePercentHealth))))
    (:then_1
      (Variables|Default|SetCurrentStamina (* (Variables|Default|GetFinalStamina) (LocalVariables|GetDeferencePercentStamina))))))

(fn HealCharacter
  (bind _finalmaxhealth (Variables|Default|GetFinalMaxHealth))
  (if (> (Variables|Default|GetCurentHealthCount) 0)
    (if (> (+ (/ _finalmaxhealth 4.0) (Variables|Default|GetCurrentHealth)) _finalmaxhealth)
      (Variables|Default|SetCurrentHealth (Variables|Default|GetFinalMaxHealth))
      (else
        (Variables|Default|SetCurrentHealth (+ (/ _finalmaxhealth 4.0) (Variables|Default|GetCurrentHealth)))))
    (Variables|Default|SetCurentHealthCount (- (Variables|Default|GetCurentHealthCount) 1))
    (return true)
    (else
      (return false))))

(fn GetDamage
  (params (Damage :type Float%20%28double-precision%29))
  (bind _finaldefense (Variables|Default|GetFinalDefense))
  (bind _output_get (Variables|Default|SetCurrentHealth (- (Variables|Default|GetCurrentHealth) (* Damage (- 1.0 (/ _finaldefense (+ _finaldefense 1e+02)))))))
  (return (> _output_get 0.0)))

(fn ConsumeStamina
  (params (Cost :type Float%20%28double-precision%29))
  (if (<= Cost (Variables|Default|GetCurrentStamina))
    (Variables|Default|SetCurrentStamina (- (Variables|Default|GetCurrentStamina) Cost))
    (Variables|Default|SetLastStaminaUse (Utilities|Time|GetGameTimeinSeconds))
    (else
      (return false))))