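; Paper2D side-scroller enemy that patrols random reachable X positions, pursues BP_Viking when seen or heard, and flips its sprite with velocity.
; On arrival, a sphere trace gates a repeating attack animation, while capsule overlap applies repeated contact damage.
; Incoming damage runs through BPHealthComponent, triggering hurt and knockback, or death with a random money reward.
; StartHitStop and EndHitStop provide a timed freeze through CustomTimeDilation.
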(event OnHearNoise(PawnSensing)
  (params (Instigator :type Pawn%20Object%20Reference) (Location :type Vector%20%28by%20ref%29 :default "0, 0, 0") (Volume :type Float%20%28single-precision%29))
  ;[0.15 0.15 0.15 0.5] Follow
  (CallFunction|AIMovement Instigator))

(event OnSeePawn(PawnSensing)
  (params (Pawn :type Pawn%20Object%20Reference))
  ;[0.15 0.15 0.15 0.5] Follow
  (CallFunction|AIMovement Pawn))

(event OnComponentBeginOverlap(CapsuleComponent)
  (params (OverlappedComponent :type Primitive%20Component%20Object%20Reference) (OtherActor :type Actor%20Object%20Reference) (OtherComp :type Primitive%20Component%20Object%20Reference) (OtherBodyIndex :type Integer) (bFromSweep :type Boolean) (SweepResult :type Hit%20Result%20Structure%20%28by%20ref%29))
  ;[0.15 0.15 0.15 0.5] OverlapedDamage
  (bind _asbp_viking (Utilities|Casting|CastToBP_Viking OtherActor))
  (Variables|Default|SetIsOverlaped true)
  (if (Math|Boolean|ANDBoolean (Variables|Default|GetIsOverlaped) (not (Variables|Default|GetIsDead?)) (not (Variables|/Game/BP/Characters/Viking/BP_Viking.BP_Viking_C|GetIsDead? _asbp_viking))) :!label _label
    (Game|Damage|ApplyDamage _asbp_viking 0.5 0 self)
    (Utilities|FlowControl|Delay 0.2)
    (goto _label)))

(event OnComponentEndOverlap(CapsuleComponent)
  (params (OverlappedComponent :type Primitive%20Component%20Object%20Reference) (OtherActor :type Actor%20Object%20Reference) (OtherComp :type Primitive%20Component%20Object%20Reference) (OtherBodyIndex :type Integer))
  ;[0.15 0.15 0.15 0.5] OverlapedDamage
  (Utilities|Casting|CastToBP_Viking OtherActor)
  (Variables|Default|SetIsOverlaped false))

(event Custom|IsInArea
  (bind _returnvalue (Transformation|GetActorLocation))
  (bind (_outhits _returnvalue_2) (Collision|MultiSphereTraceForObjects _returnvalue _returnvalue 6e+01 (Utilities|Array|MakeArray "ObjectTypeQuery3") false 0 "None"))
  (if _returnvalue_2
    (for _array_element _outhits
      (Utilities|Casting|CastToBP_Viking (.HitActor (Collision|BreakHitResult _array_element))
        (:then
          (Variables|Default|SetIsInArea? true))
        (:CastFailed
          (Variables|Default|SetIsInArea? false))))
    (else
      (Variables|Default|SetIsInArea? false))))

(event Custom|Moving
  (bind _returnvalue (Transformation|GetActorLocation))
  (bind (_x _y _z) (Math|Vector|BreakVector _returnvalue))
  ;[0.15 0.15 0.15 0.5] Patrol Location
  (if (and (Variables|Default|GetCanMoving?) (not (Variables|Default|GetIsDead?)))
    (AI|AIMoveTo self (Math|Vector|MakeVector (.x (.RandomLocation (AI|Navigation|GetRandomReachablePointinRadius _returnvalue 5e+02 0 0))) _y _z) 0 5.0 false
      (:OnSuccess
        (Utilities|FlowControl|Delay 2.0)
        (CallFunction|Moving)))))

(event Custom|Attack
  (if (Math|Boolean|ANDBoolean (Variables|Default|GetCanMoving?) (not (Variables|Default|GetIsDead?)) (Variables|Default|GetIsInArea?))
    (Components|Movement|StopMovementImmediately (Variables|Character|GetCharacterMovement))
    (Variables|Default|SetCanMoving? false)
    (Variables|Default|SetIsAttacking true)
    (|PlayAnimationOverridewithCallbacks (Variables|/Script/PaperZD.PaperZDAnimationComponent|GetAnimInstance (Variables|Default|GetAnimationComponent)) (Variables|Default|GetAttack) "DefaultSlot" 1.0 0.0
      (:OnCompleted
        (CallFunction|IsinArea)
        (Utilities|FlowControl|Delay 1.0)
        (Variables|Default|SetCanMoving? true)
        (Variables|Default|SetIsAttacking false)
        (CallFunction|Attack)))))

(event Custom|AI%20Movement
  (params (Object :type Object%20Object%20Reference))
  ;[0.15 0.15 0.15 0.5] Follow
  (bind _asbp_viking (Utilities|Casting|CastToBP_Viking Object))
  (if (Math|Boolean|ANDBoolean (not (Variables|/Game/BP/Characters/Viking/BP_Viking.BP_Viking_C|GetIsDead? _asbp_viking)) (not (Variables|Default|GetIsDead?)) (Variables|Default|GetCanMoving?))
    (AI|AIMoveTo self (Math|Vector|MakeVector 0.0 0.0 0.0) _asbp_viking 15.0 true
      (:OnSuccess
        (CallFunction|IsinArea)
        (CallFunction|Attack))
      (:OnFail
        (Utilities|FlowControl|RetriggerableDelay 2.0)
        (CallFunction|Moving)))))

(event Custom|AddKnockback
  (params (PointX :type Float%20%28double-precision%29))
  (bind _returnvalue (Transformation|GetActorForwardVector))
  (Variables|Default|SetIsKnockbacking true)
  (Character|LaunchCharacter (Math|Vector|MakeVector (select (> (.x (Transformation|GetWorldLocation (Variables|Default|GetSprite))) PointX) (* (.x _returnvalue) 5e+02) (* (.x _returnvalue) -5e+02)) 0.0 2e+01) true false)
  (Utilities|FlowControl|Delay 0.1)
  (Variables|Default|SetIsKnockbacking true))

(event Custom|AddRotation
  (params (PointX :type Float%20%28double-precision%29))
  (bind _sprite (Variables|Default|GetSprite))
  (bind _charactermovement (Variables|Character|GetCharacterMovement))
  (bind _sprite_2 (Variables|Default|GetSprite))
  (bind _returnvalue (Transformation|GetWorldScale _sprite_2))
  (bind _returnvalue_2 (Transformation|GetWorldScale _sprite))
  (bind _velocity (Variables|/Script/Engine.MovementComponent|GetVelocity _charactermovement))
  (if (and (> (Math|Float|Absolute(Float) (.x _velocity)) 5.0) (not (Variables|Default|GetIsKnockbacking)))
    (if (> (.x _velocity) 0.0)
      (Transformation|SetWorldScale3D _sprite_2 (Math|Vector|MakeVector 1.0 (.y _returnvalue) (.z _returnvalue)))
      (else
        (Transformation|SetWorldScale3D _sprite (Math|Vector|MakeVector -1.0 (.y _returnvalue_2) (.z _returnvalue_2)))))))

(event EventBeginPlay
  (Default|CallOnSpawned)
  (CallFunction|Moving))

(event Collision|EventActorBeginOverlap
  (params (OtherActor :type Actor%20Object%20Reference)))

(event EventTick
  (params (DeltaSeconds :type Float%20%28single-precision%29))
  (CallFunction|AddRotation 0.0))

(event Game|Damage|EventAnyDamage
  (params (Damage :type Float%20%28single-precision%29) (DamageType :type Damage%20Type%20Object%20Reference) (InstigatedBy :type Controller%20Object%20Reference) (DamageCauser :type Actor%20Object%20Reference))
  (bind _returnvalue (Game|Player|GetPlayerPawn 0))
  (bind _returnvalue_2 (Transformation|GetActorLocation _returnvalue))
  ;[0.15 0.15 0.15 0.5] OnAnyDamge
  (if (and (> (Variables|/Game/BP/Component/BP_HealthComponent.BP_HealthComponent_C|Gethealth (Variables|Default|GetBP_HealthComponent)) 0.0) (not (Variables|Default|GetIsDead?)))
    (Variables|Default|SetCanMoving? false)
    (bind _islive_ (Default|GetDamage (Variables|Default|GetBP_HealthComponent) Damage))
    (if _islive_
      (|PlayAnimationOverridewithCallbacks (Variables|/Script/PaperZD.PaperZDAnimationComponent|GetAnimInstance (Variables|Default|GetAnimationComponent)) (Variables|Default|GetHurt) "DefaultSlot" 1.0 0.0
        (:then
          (Utilities|FlowControl|Delay 0.1)
          (CallFunction|AddRotation (.x _returnvalue_2))
          (CallFunction|AddKnockback (.x _returnvalue_2)))
        (:OnCompleted
          (Variables|Default|SetCanMoving? true)))
      (else
        (Variables|Default|SetIsDead? true)
        (|PlayAnimationOverridewithCallbacks (Variables|/Script/PaperZD.PaperZDAnimationComponent|GetAnimInstance (Variables|Default|GetAnimationComponent)) (Variables|Default|GetDeath) "DefaultSlot" 1.0 0.0
          (:OnCompleted
            (bind _asbp_viking (Utilities|Casting|CastToBP_Viking (Game|Player|GetPlayerPawn 0)))
            (Variables|/Game/BP/Characters/Viking/BP_Viking.BP_Viking_C|SetMoney _asbp_viking (+ (Variables|/Game/BP/Characters/Viking/BP_Viking.BP_Viking_C|GetMoney _asbp_viking) (Math|Random|RandomIntegerinRange 5 20)))
            (Actor|DestroyActor)
            (Default|CallDeathEvent)))))))

(event EventPossessed
  (params (NewController :type Controller%20Object%20Reference))
  (Default|CallOnSpawned)
  (CallFunction|Moving))

(fn ConstructionScript)

(fn StartHitStop
  (params (Time :type Float%20%28single-precision%29))
  (Variables|Default|SetCustomTimeDilation 0.0)
  (Utilities|Time|SetTimerbyFunctionName 0 "EndHitStop" Time))

(fn EndHitStop
  (Variables|Default|SetCustomTimeDilation 1.0))