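; Mimic boss that the Viking player talks to, then fights once a dialogue trigger starts the battle.
; It loops its attack animation with random pauses while Tick checks health against quarter-based stage thresholds.
; Each threshold makes it invulnerable and spawns two random minions, whose death events restore damage.
; Death switches it to a second dialogue, whose End trigger fades out and opens the Cut2 level.
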(event OnComponentBeginOverlap(CapsuleComponent)
  (params (OverlappedComponent :type Primitive%20Component%20Object%20Reference) (OtherActor :type Actor%20Object%20Reference) (OtherComp :type Primitive%20Component%20Object%20Reference) (OtherBodyIndex :type Integer) (bFromSweep :type Boolean) (SweepResult :type Hit%20Result%20Structure%20%28by%20ref%29))
  (if (not (Variables|Default|GetInFight?))
    (Utilities|Casting|CastToBP_Viking OtherActor)
    (Rendering|SetVisibility (Variables|Default|GetWidget) true false)))

(event OnComponentEndOverlap(CapsuleComponent)
  (params (OverlappedComponent :type Primitive%20Component%20Object%20Reference) (OtherActor :type Actor%20Object%20Reference) (OtherComp :type Primitive%20Component%20Object%20Reference) (OtherBodyIndex :type Integer))
  (if (not (Variables|Default|GetInFight?))
    (Utilities|Casting|CastToBP_Viking OtherActor)
    (Rendering|SetVisibility (Variables|Default|GetWidget) false false)))

(event Custom|Attack
  (if (not (Variables|Default|GetDead?))
    (Variables|Default|SetIsAttacking? true)
    (|PlayAnimationOverridewithCallbacks (Variables|/Script/PaperZD.PaperZDAnimationComponent|GetAnimInstance (Variables|Default|GetAnimationComponent)) "/Game/BP/Characters/enemy/Mimic/AnimSequences/attack.attack" "DefaultSlot" 1.0 0.0
      (:OnCompleted
        (Variables|Default|SetIsAttacking? false)
        (Utilities|FlowControl|Delay (Math|Conversions|ToFloat(Integer) (Math|Random|RandomIntegerinRange 2 8)))
        (CallFunction|Attack)))))

(event Custom|Death
  (bind _bp_dialoguecomponent (Variables|Default|GetBP_DialogueComponent))
  (Variables|Default|SetDead? true)
  (Class|PaperZDAnimInstance|JumptoNode (Variables|/Script/PaperZD.PaperZDAnimationComponent|GetAnimInstance (Variables|Default|GetAnimationComponent)) "Death" "None")
  (Variables|/Game/BP/Component/BP_DialogueComponent.BP_DialogueComponent_C|SetIs%20Dialogue%20End? _bp_dialoguecomponent false)
  (Variables|/Game/BP/Component/BP_DialogueComponent.BP_DialogueComponent_C|SetName _bp_dialoguecomponent "Мимик")
  (Variables|/Game/BP/Component/BP_DialogueComponent.BP_DialogueComponent_C|SetRowName (Variables|Default|GetBP_DialogueComponent) "1")
  (Variables|/Game/BP/Component/BP_DialogueComponent.BP_DialogueComponent_C|SetDataTable (Variables|Default|GetBP_DialogueComponent) "/Game/BP/Dialogue/Mimic2.Mimic2")
  (Rendering|SetVisibility (Variables|Default|GetWidget) true false)
  (Variables|Default|SetInFight? false))

(event EventBeginPlay
  (Utilities|FlowControl|Sequence))

(event EventInteract
  (params (PlayerRef :type BP%20Viking%20Object%20Reference) (Owner :type Object%20Object%20Reference))
  (if (not (Variables|Default|GetInFight?))
    (Default|Interact (Variables|Default|GetBP_DialogueComponent) PlayerRef self)))

(event EventTick
  (params (DeltaSeconds :type Float%20%28single-precision%29))
  (if (Variables|Default|GetInFight?)
    (|SpawActors)))

(event Game|Damage|EventAnyDamage
  (params (Damage :type Float%20%28single-precision%29) (DamageType :type Damage%20Type%20Object%20Reference) (InstigatedBy :type Controller%20Object%20Reference) (DamageCauser :type Actor%20Object%20Reference))
  (if (and (Variables|Default|GetCanDamage?) (Variables|Default|GetInFight?))
    (bind _islive_ (Default|GetDamage (Variables|Default|GetBP_HealthComponent) Damage))
    (if _islive_
      (if (not (Variables|Default|GetIsAttacking?))
        (Class|PaperZDAnimInstance|JumptoNode (Variables|/Script/PaperZD.PaperZDAnimationComponent|GetAnimInstance (Variables|Default|GetAnimationComponent)) "Hurt" "None"))
      (else
        (CallFunction|Death)))))

(event EventTrigger
  (params (TriggerName :type Name :default "None") (Row%20Name :type Name :default "None") (Data%20Table :type Data%20Table%20Object%20Reference))
  (if (== TriggerName "Name")
    (Variables|/Game/BP/Component/BP_DialogueComponent.BP_DialogueComponent_C|SetName (Variables|Default|GetBP_DialogueComponent) "Мимик")
    (elif (== TriggerName "Name1")
      (Variables|/Game/BP/Component/BP_DialogueComponent.BP_DialogueComponent_C|SetName (Variables|Default|GetBP_DialogueComponent) "Фрейвар")
      (elif (== TriggerName "Fight")
        (Variables|Default|SetInFight? true)
        (Default|EndInteract (Variables|Default|GetBP_DialogueComponent))
        (Utilities|FlowControl|Delay 1.0)
        (Default|CallFight)
        (Audio|PlaySound2D "/Game/Assets/Sound/Music/bossMusic_Cue.bossMusic_Cue" 1.0 1.0 0.0 0 0)
        (CallFunction|Attack)
        (bind _asbp_viking (Utilities|Casting|CastToBP_Viking (Game|Player|GetPlayerPawn 0)))
        (Variables|/Game/BP/Characters/Viking/BP_Viking.BP_Viking_C|SetIsInBattle? _asbp_viking true)
        (Rendering|SetVisibility (Variables|Default|GetWidget) false false)
        (elif (== TriggerName "End")
          (CameraFades|StartCameraFade :self (Game|GetPlayerCameraManager 0) :ToAlpha 1.0 :Duration 1.0 :bHoldWhenFinished true)
          (bind _asbp_viking_2 (Utilities|Casting|CastToBP_Viking (Game|Player|GetPlayerPawn 0)))
          (Widget|SetVisibility (Variables|/Game/BP/Characters/Viking/BP_Viking.BP_Viking_C|GetUI _asbp_viking_2) "Hidden")
          (Utilities|FlowControl|Delay 1.0)
          (Game|OpenLevel(byObjectReference) "/Game/Maps/Cutscene/Cut2.Cut2"))))))

(fn ConstructionScript)

(event Custom|DeathMim
  (Variables|Default|SetEnemyCount (- (Variables|Default|GetEnemyCount) 1))
  (if (<= (Variables|Default|GetEnemyCount) 0)
    (Class|PaperZDAnimInstance|JumptoNode (Variables|/Script/PaperZD.PaperZDAnimationComponent|GetAnimInstance (Variables|Default|GetAnimationComponent)) "Angry" "None")
    (Variables|Default|SetCanDamage? true)))