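; BP_NPC is a non-player character the player's Viking can talk to.
; A sphere overlap with BP_Viking shows or hides the interaction widget, and Interact and EndInteract forward to the dialogue component.
; On Tick, when the level is "Test" and the dialogue reaches row "7", it creates the shop widget once and adds it to the viewport.
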(event OnComponentBeginOverlap(Sphere)
  (params (OverlappedComponent :type Primitive%20Component%20Object%20Reference) (OtherActor :type Actor%20Object%20Reference) (OtherComp :type Primitive%20Component%20Object%20Reference) (OtherBodyIndex :type Integer) (bFromSweep :type Boolean) (SweepResult :type Hit%20Result%20Structure%20%28by%20ref%29))
  (Utilities|Casting|CastToBP_Viking OtherActor)
  (Rendering|SetVisibility (Variables|Default|GetWidgetInteraction) true false))

(event OnComponentEndOverlap(Sphere)
  (params (OverlappedComponent :type Primitive%20Component%20Object%20Reference) (OtherActor :type Actor%20Object%20Reference) (OtherComp :type Primitive%20Component%20Object%20Reference) (OtherBodyIndex :type Integer))
  (Utilities|Casting|CastToBP_Viking OtherActor)
  (Rendering|SetVisibility (Variables|Default|GetWidgetInteraction) false false))

(event EventBeginPlay)

(event Collision|EventActorBeginOverlap
  (params (OtherActor :type Actor%20Object%20Reference)))

(event EventTick
  (params (DeltaSeconds :type Float%20%28single-precision%29))
  (bind _returnvalue (Game|GetCurrentLevelName true))
  (if (== (Utilities|String|StringToName _returnvalue) "Test")
    (if (== (Variables|/Game/BP/Component/BP_DialogueComponent.BP_DialogueComponent_C|GetRowName (Variables|Default|GetBP_DialogueComponent)) "7")
      (Utilities|IsValid (Variables|Default|GetShop)
        (:Is%20Not%20Valid
          (bind _returnvalue_2 (UserInterface|CreateWidget "/Game/BP/Widget/WB_Shop.WB_Shop_C" (Game|GetPlayerController 0)))
          (Variables|Default|SetShop _returnvalue_2)
          (UserInterface|Viewport|AddtoViewport _returnvalue_2 0))))))

(event EventInteract
  (params (PlayerRef :type BP%20Viking%20Object%20Reference))
  (Class|BPIInteract|Interact(Message) (Variables|Default|GetBP_DialogueComponent) PlayerRef))

(event EventEndInteract
  (Class|BPIInteract|EndInteract(Message) (Variables|Default|GetBP_DialogueComponent)))

(fn ConstructionScript)