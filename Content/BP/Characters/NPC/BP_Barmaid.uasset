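; BP_Barmaid is an NPC Blueprint for a barmaid with dialogue and a shop.
; On BeginPlay it sets the dialogue display name to "Каиса" if the dialogue component's row number has reached a threshold.
; Its Trigger event responds by name: "Shop" creates the shop through BPShopComponent and passes the row to OptionSelected on BPDialogueComponent, while "Name" sets that same display name.
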(event EventBeginPlay
  (|CallParentFunction)
  (if (>= (Math|Conversions|ToInteger(Byte) (Utilities|String|ToString(Name) (Variables|/Game/BP/Component/BP_DialogueComponent.BP_DialogueComponent_C|GetRowName (Variables|Default|GetBP_DialogueComponent)))) 4)
    (Variables|/Game/BP/Component/BP_DialogueComponent.BP_DialogueComponent_C|SetName (Variables|Default|GetBP_DialogueComponent) "Каиса")))

(event Collision|EventActorBeginOverlap
  (params (OtherActor :type Actor%20Object%20Reference))
  (|CallParentFunction OtherActor) ; This node is disabled and will not be called.\nDrag off pins to build functionality.
)

(event EventTick
  (params (DeltaSeconds :type Float%20%28single-precision%29)))

(event EventTrigger
  (params (TriggerName :type Name :default "None") (Row%20Name :type Name :default "None") (Data%20Table :type Data%20Table%20Object%20Reference))
  (if (== TriggerName "Shop")
    (Default|CreateShop (Variables|Default|GetBP_ShopComponent) true)
    (Default|OptionSelected (Variables|Default|GetBP_DialogueComponent) Data%20Table Row%20Name)
    (elif (== TriggerName "Name")
      (Variables|/Game/BP/Component/BP_DialogueComponent.BP_DialogueComponent_C|SetName (Variables|Default|GetBP_DialogueComponent) "Каиса"))))

(fn ConstructionScript
  (|CallParentFunction))