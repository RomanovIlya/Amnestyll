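; BP_Blacksmith is an NPC Blueprint for a blacksmith that can open a shop from dialogue.
; Its Trigger event checks for the "Shop" trigger name, then has the shop component create the shop and passes the row and data table to the dialogue component as the selected option.
; BeginPlay, overlap and Tick are unused, and the construction script only calls the parent.
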(event EventBeginPlay
  (|CallParentFunction) ; This node is disabled and will not be called.\nDrag off pins to build functionality.
)

(event Collision|EventActorBeginOverlap
  (params (OtherActor :type Actor%20Object%20Reference))
  (|CallParentFunction OtherActor) ; This node is disabled and will not be called.\nDrag off pins to build functionality.
)

(event EventTick
  (params (DeltaSeconds :type Float%20%28single-precision%29)))

(event EventTrigger
  (params (TriggerName :type Name :default "None") (Row%20Name :type Name :default "None") (Data%20Table :type Data%20Table%20Object%20Reference))
  (if (== TriggerName "Shop")
    (Default|CreateShop (Variables|Default|GetBP_ShopComponent) true)
    (Default|OptionSelected (Variables|Default|GetBP_DialogueComponent) Data%20Table Row%20Name)))

(fn ConstructionScript
  (|CallParentFunction))